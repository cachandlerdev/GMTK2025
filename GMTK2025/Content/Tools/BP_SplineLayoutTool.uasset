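; Spline layout tool actor that fills a spline with instanced copies of a chosen mesh in the Construction Script.
; Spacing comes from the mesh's X bounds plus an offset, and the spline length determines the instance count.
; Each instance aims its selected forward axis at the next spline point.
; Unseeded random location and rotation jitter is added, so the layout varies on each reconstruction.
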(event EventBeginPlay)

(event Collision|EventActorBeginOverlap
  (params (OtherActor :type Actor%20Object%20Reference)))

(event EventTick
  (params (DeltaSeconds :type Float%20%28single-precision%29)))

(fn ConstructionScript
  (bind _placedmesh (Variables|SplineLayout|GetPlacedMesh))
  (bind _returnvalue (StaticMesh|GetBoundingBox _placedmesh))
  (bind (_min _max) (Utilities|Struct|BreakBox _returnvalue))
  (Components|StaticMesh|SetStaticMesh (Variables|Default|GetInstancedStaticMesh) _placedmesh)
  (bind _output_get (Variables|SplineLayout|SetSpacing (+ (.X (Math|Vector|BreakVector (- _max _min))) (Variables|SplineLayout|GetDistanceOffset))))
  (bind _output_get_2 (LocalVariables|SetNumberOfInstances (Math|Float|Floor (/ (Spline|GetSplineLength (Variables|Default|GetSpline)) _output_get))))
  (for _index (range 0 _output_get_2)
    (Components|InstancedStaticMesh|AddInstance (Variables|Default|GetInstancedStaticMesh) (Math|Transform|MakeTransform (.OutLocation (CallFunction|AddJitter (CallFunction|GetLocationatIndex _index) (CallFunction|GetRotationbyAxis (- (CallFunction|GetLocationatIndex (+ _index 1)) (CallFunction|GetLocationatIndex _index))))) (.OutRotation (CallFunction|AddJitter (CallFunction|GetLocationatIndex _index) (CallFunction|GetRotationbyAxis (- (CallFunction|GetLocationatIndex (+ _index 1)) (CallFunction|GetLocationatIndex _index)))))) false)))

(fn GetLocationatIndex
  (params (Index :type Integer))
  (return (Spline|GetLocationatDistanceAlongSpline (Variables|Default|GetSpline) (* Index (Variables|SplineLayout|GetSpacing)) "Local")))

(fn AddJitter
  (params (Location :type Vector) (Rotation :type Rotator))
  (return (+ Location (* (Math|Random|RandomFloatinRange 0.0 (Variables|SplineLayout|GetMaxLocationJitter)) (Math|Random|RandomUnitVector))) (Math|Rotator|CombineRotators Rotation (* (Math|Random|RandomRotator false) (Math|Random|RandomFloatinRange 0.0 (Variables|SplineLayout|GetMaxRotationJitter))))))

(fn GetRotationbyAxis
  (params (GetLocation :type Vector))
  (switch Utilities|FlowControl|Switch|SwitchonEAxis (Variables|SplineLayout|GetForwardAxis)
    (:None
      _)
    (:X
      _)
    (:Y
      (return (Math|Rotator|MakeRotfromY GetLocation)))
    (:Z
      (return (Math|Rotator|MakeRotfromZ GetLocation))))
  (return (Math|Rotator|MakeRotfromX GetLocation)))