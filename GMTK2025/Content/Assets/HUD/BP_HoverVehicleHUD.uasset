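; BP_HoverVehicleHUD is the hover vehicle HUD that creates the on-screen widgets for speed, player position, loop info and inventory.
; On BeginPlay it calls CreateWidgets, which creates each widget, stores it in a variable and adds it to the viewport.
; Each widget is set to HitTestInvisible so it is visible without intercepting pointer input.
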(event EventBeginPlay
  (CallFunction|CreateWidgets))

(fn ConstructionScript)

(fn CreateWidgets
  (Utilities|FlowControl|Sequence
    (:then_0
      (bind _returnvalue (UserInterface|CreateWidget "/Game/Assets/HUD/WBP_Speed.WBP_Speed_C"))
      (bind _output_get (Variables|Default|SetSpeedWidget _returnvalue))
      (UserInterface|Viewport|AddtoViewport _output_get 0)
      (Widget|SetVisibility _output_get "HitTestInvisible"))
    (:then_1
      (bind _returnvalue_2 (UserInterface|CreateWidget "/Game/Assets/HUD/WBP_PlayerPosition.WBP_PlayerPosition_C"))
      (bind _output_get_2 (Variables|Default|SetPlayerPositionWidget _returnvalue_2))
      (UserInterface|Viewport|AddtoViewport _output_get_2 0)
      (Widget|SetVisibility _output_get_2 "HitTestInvisible"))
    (:then_2
      (bind _returnvalue_3 (UserInterface|CreateWidget "/Game/Assets/HUD/WBP_LoopInfo.WBP_LoopInfo_C"))
      (bind _output_get_3 (Variables|Default|SetLoopInfoWidget _returnvalue_3))
      (UserInterface|Viewport|AddtoViewport _output_get_3 0)
      (Widget|SetVisibility _output_get_3 "HitTestInvisible"))
    (:then_3
      (bind _returnvalue_4 (UserInterface|CreateWidget "/Game/Assets/HUD/WBP_Inventory.WBP_Inventory_C"))
      (bind _output_get_4 (Variables|Default|SetInventoryWidget _returnvalue_4))
      (UserInterface|Viewport|AddtoViewport _output_get_4 0)
      (Widget|SetVisibility _output_get_4 "HitTestInvisible"))))